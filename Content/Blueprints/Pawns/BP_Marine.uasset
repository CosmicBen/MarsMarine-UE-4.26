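; BP_Marine is the player pawn for a twin-stick shooter, with world-axis movement, health, a kill counter and a HUD created at BeginPlay.
; Each tick sets control rotation from thumbstick direction or smoothed mouse velocity, depending on whether the last key pressed was gamepad.
; Firing loops a timer-driven line trace from the muzzle along that rotation, applying damage with effects and sound.
; Zero health marks it dead, disabling movement, aiming and firing.
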(event EventBeginPlay
  (bind _returnvalue (UserInterface|CreateWidget "/Game/UI/W_PlayerHud.W_PlayerHud_C" 0 self))
  (UserInterface|Viewport|AddtoViewport _returnvalue 0))

(event Collision|EventActorBeginOverlap
  (params (OtherActor :type Actor%20Object%20Reference)))

(event EventTick
  (params (DeltaSeconds :type Float%20%28single-precision%29))
  (CallFunction|UpdatePlayerAim))

(event Game|Damage|EventAnyDamage
  (params (Damage :type Float%20%28single-precision%29) (DamageType :type Damage%20Type%20Object%20Reference) (InstigatedBy :type Controller%20Object%20Reference) (DamageCauser :type Actor%20Object%20Reference))
  (if (CallFunction|IsAlive)
    (bind _health (CallFunction|DecreaseHealth Damage))
    (bind _output_get (Variables|PlayerProperties|SetbIsDead (Math|Float|NearlyEqual(Float) _health 0.0 1e-06)))
    (if _output_get
      (Utilities|FlowControl|DoOnce false
        (:Completed
          (CallFunction|StopFiringWeapon))))))

(event Input|ActionEvents|InputActionFireWeapon
  (params (Key :type Key%20Structure :default "None"))
  (:Pressed
    (CallFunction|StartFiringWeapon))
  (:Released
    (if (CallFunction|IsAlive)
      (CallFunction|StopFiringWeapon))))

(event Input|AxisEvents|InputAxisMoveForward
  (params (AxisValue :type Float%20%28single-precision%29))
  (if (CallFunction|IsAlive)
    (Pawn|Input|AddMovementInput "1.000000, 0, 0" AxisValue false)))

(event Input|AxisEvents|InputAxisMoveRight
  (params (AxisValue :type Float%20%28single-precision%29))
  (if (CallFunction|IsAlive)
    (Pawn|Input|AddMovementInput "0.000000,1.000000, 0" AxisValue false)))

(event Input|KeyboardEvents|AnyKey
  (params (Key :type Key%20Structure :default "None"))
  (:Pressed
    (Variables|ThumbstickInput|SetbIsGamepadActive (Class|KismetInputLibrary|KeyIsGamepadKey Key))))

(fn ConstructionScript)

(fn UpdatePlayerAim
  (if (CallFunction|IsAlive)
    (if (Variables|ThumbstickInput|GetbIsGamepadActive)
      (ThumbstickInput|UpdateThumbstickAim)
      (else
        (MouseInput|UpdateMouseAim)))))

(fn IsThumbstickAboveDeadzone
  (return (> (Class|KismetMathLibrary|VSize2DSquared (Math|Vector2D|MakeVector2D (Input|AxisValues|GetThumbstickAimUp) (Input|AxisValues|GetThumbstickAimRight))) (Variables|ThumbstickInput|GetThumbstickDeadzone))))

(fn GetMouseVelocity
  (bind _returnvalue (Game|GetPlayerController 0))
  (bind (_deltax _deltay) (Class|PlayerController|GetInputMouseDelta _returnvalue))
  (return (/ (Math|Vector2D|MakeVector2D _deltax _deltay) (Utilities|Time|GetWorldDeltaSeconds))))

(fn IsMouseAboveDeadzone
  (return (> (Class|KismetMathLibrary|VSize2DSquared (MouseInput|GetMouseVelocity)) (Variables|ThumbstickInput|GetThumbstickDeadzone))))

(fn UpdateMouseAim
  (if (MouseInput|IsMouseAboveDeadzone)
    (Pawn|SetControlRotation (Game|GetPlayerController 0) (MouseInput|GetMouseAimDirection))
    (return)))

(fn GetMouseAimDirection
  (bind _velocity (MouseInput|GetMouseVelocity))
  (return (Math|Interpolation|RInterpTo (Pawn|GetControlRotation (Game|GetPlayerController 0) :!class /Script/Engine.Controller) (Math|Rotator|MakeRotator 0.0 0.0 (Class|KismetMathLibrary|DegAtan2 (.x _velocity) (.y _velocity))) (Utilities|Time|GetWorldDeltaSeconds) (Variables|MouseInput|GetMouseSmoothingStrength))))

(fn UpdateThumbstickAim
  (if (ThumbstickInput|IsThumbstickAboveDeadzone)
    (Pawn|SetControlRotation (Game|GetPlayerController 0) (ThumbstickInput|GetThumbstickAimDirection))
    (return)))

(fn GetThumbstickAimDirection
  (return (Math|Rotator|MakeRotator 0.0 0.0 (Class|KismetMathLibrary|DegAtan2 (Input|AxisValues|GetThumbstickAimUp) (Input|AxisValues|GetThumbstickAimRight)))))

(fn StartFiringWeapon
  (if (CallFunction|IsAlive)
    (Components|Activation|Activate (Variables|Default|GetP_AssaultRifle_MF) false)
    (bind _returnvalue (Audio|SpawnSound2D "/Game/Sounds/Weapon_AssaultRifle/Stereo/RifleFireLoop_Cue.RifleFireLoop_Cue" 1.0 1.0 0.0 0))
    (Variables|Default|SetWeaponFireSound _returnvalue)
    (CallFunction|WeaponTrace)
    (Utilities|Time|SetTimerbyFunctionName 0 "WeaponTrace" (Variables|PlayerProperties|GetWeaponFireRate) true)))

(fn StopFiringWeapon
  (bind _weaponfiresound (Variables|Default|GetWeaponFireSound))
  (Components|Activation|Deactivate (Variables|Default|GetP_AssaultRifle_MF))
  (Utilities|IsValid _weaponfiresound
    (:Is%20Valid
      (Audio|Components|Audio|Stop _weaponfiresound)
      (Utilities|Time|ClearTimerbyFunctionName 0 "WeaponTrace")
      (Audio|SpawnSound2D "/Game/Sounds/Weapon_AssaultRifle/Stereo/RifleFireStop_Cue.RifleFireStop_Cue" 1.0 1.0 0.0 0))))

(fn DecreaseHealth
  (params (DamageAmount :type Float%20%28single-precision%29))
  (bind _output_get (Variables|PlayerProperties|SetHealth (Math|Float|Clamp(Float) (- (Variables|PlayerProperties|GetHealth) DamageAmount) 0.0 1e+02)))
  (return _output_get))

(fn IsAlive
  (return (not (Variables|PlayerProperties|GetbIsDead))))

(fn WeaponTrace
  (bind _outhit (Collision|LineTraceByChannel (CallFunction|GetWeaponTraceStartLocation) (CallFunction|GetWeaponTraceEndLocation) "TraceTypeQuery1" false 0 "None"))
  (if (.bBlockingHit (Collision|BreakHitResult _outhit))
    (Game|Damage|ApplyDamage (.HitActor (Collision|BreakHitResult _outhit)) (Variables|PlayerProperties|GetDamagePerShot) 0 0)
    (CallFunction|SpawnImpactHit (.Location (Collision|BreakHitResult _outhit)))))

(fn GetWeaponTraceStartLocation
  (return (Transformation|GetSocketLocation (Variables|Default|GetRifle) "MuzzleFlashSocket")))

(fn GetWeaponTraceEndLocation
  (return (+ (CallFunction|GetWeaponTraceStartLocation) (* (Math|Vector|GetForwardVector (Pawn|GetControlRotation :!class /Script/Engine.Pawn)) (Variables|PlayerProperties|GetWeaponRange)))))

(fn IncreaseKills
  (Math|Integer|IncrementInt (Variables|PlayerProperties|GetKills)
    (:%20%20
      (return))))

(fn SpawnImpactHit
  (params (HitLocation :type Vector))
  (Effects|SpawnEmitteratLocation "/Game/Effects/Weapons/Impacts/P_AssaultRifle_IH.P_AssaultRifle_IH" HitLocation))

(fn AddHealth
  (params (HealthToAdd :type Float%20%28single-precision%29))
  (Variables|PlayerProperties|SetHealth (Math|Float|Clamp(Float) (+ HealthToAdd (Variables|PlayerProperties|GetHealth)) 0.0 1e+02)))

(fn IsHealthFull
  (return (Math|Float|NearlyEqual(Float) (Variables|PlayerProperties|GetHealth) 1e+02 1e-06)))