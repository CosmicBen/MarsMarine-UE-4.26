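; BP_Alien is an enemy AI character that chases the player and attacks at close range.
; A looping AIMoveTo drives pursuit, while Tick checks range and pauses movement during the attack montage.
; DamagePlayer applies hit damage but has no caller in this Blueprint.
; At zero health, it disables movement and collision, credits a BP_Marine kill, notifies the game mode, then destroys itself after a delay.
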(event EventBeginPlay
  (AI|AIMoveTo self "0, 0, 0" (Game|GetPlayerCharacter 0) 5.0 false :!label _label
    (:OnSuccess
      _)
    (:OnFail
      _))
  (Utilities|FlowControl|Delay 0.2)
  (if (CallFunction|IsAlive)
    (goto _label)))

(event EventTick
  (params (DeltaSeconds :type Float%20%28single-precision%29))
  (if (Math|Boolean|ANDBoolean (CallFunction|IsAlive) (CallFunction|IsWithinAttackRange) (not (CallFunction|IsAttacking)))
    (CallFunction|DeactivateAiMovement)
    (Animation|Montage|PlayMontage (Variables|Character|GetMesh) "/Game/Characters/Enemy_Great_Spider/Animations/AlienAttack1.AlienAttack1"
      (:OnCompleted
        (CallFunction|ActivateAiMovement)))))

(event Game|Damage|EventAnyDamage
  (params (Damage :type Float%20%28single-precision%29) (DamageType :type Damage%20Type%20Object%20Reference) (InstigatedBy :type Controller%20Object%20Reference) (DamageCauser :type Actor%20Object%20Reference))
  (if (CallFunction|IsAlive)
    (bind _health (CallFunction|DecreaseHealth Damage))
    (if (Math|Float|NearlyEqual(Float) _health 0.0 1e-06)
      (CallFunction|KillAi)
      (Utilities|FlowControl|Delay 3.0)
      (Actor|DestroyActor))))

(fn ConstructionScript)

(fn IsWithinAttackRange
  (return (< (Transformation|GetDistanceTo (Game|Player|GetPlayerPawn 0)) (Variables|Default|GetAttackRange))))

(fn IsAttacking
  (return (Animation|Montage|MontageIsPlaying (Components|SkeletalMesh|GetAnimInstance (Variables|Character|GetMesh)) "/Game/Characters/Enemy_Great_Spider/Animations/AlienAttack1.AlienAttack1")))

(fn ActivateAiMovement
  (Components|Activation|Activate (Variables|Character|GetCharacterMovement) false))

(fn DeactivateAiMovement
  (bind _charactermovement (Variables|Character|GetCharacterMovement))
  (Components|Movement|StopMovementImmediately _charactermovement)
  (Components|Activation|Deactivate _charactermovement))

(fn DamagePlayer
  (if (CallFunction|IsAlive)
    (Game|Damage|ApplyDamage (Game|GetPlayerCharacter 0) (Variables|Default|GetDamagePerHit) 0 0)))

(fn DecreaseHealth
  (params (Damage :type Float%20%28single-precision%29))
  (bind _output_get (Variables|Default|SetHealth (- (Variables|Default|GetHealth) Damage)))
  (return (Math|Float|Clamp(Float) _output_get 0.0 1e+02)))

(fn KillAi
  (Variables|Default|SetbIsDead true)
  (CallFunction|DeactivateAiMovement)
  (Collision|SetActorEnableCollision false)
  (bind _asbp_marine (Utilities|Casting|CastToBP_Marine (Game|GetPlayerCharacter 0)))
  (Default|IncreaseKills _asbp_marine)
  (bind _asbp_mars_marine_game_mode (Utilities|Casting|CastToBP_MarsMarine_GameMode (Game|GetGameMode)))
  (Default|RegisterAlienDeath _asbp_mars_marine_game_mode self))

(fn IsAlive
  (return (not (Variables|Default|GetbIsDead))))

(fn DeactiveA
  (Components|Activation|Deactivate (Variables|Character|GetCharacterMovement)))