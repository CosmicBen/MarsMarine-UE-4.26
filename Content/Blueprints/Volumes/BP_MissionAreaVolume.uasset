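; BP_MissionAreaVolume is a trigger volume that bounds the mission area and punishes the player for leaving it.
; When a BP_Marine exits, it sets that marine's OutsideMissionArea flag and starts a KillPlayer timer of SecondsBeforePlayerDeath.
; Re-entering clears the flag and cancels the timer.
; On expiry, KillPlayer applies massive damage to player character 0, regardless of which marine left.
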(event Collision|EventActorBeginOverlap
  (params (OtherActor :type Actor%20Object%20Reference))
  (bind _asbp_marine (Utilities|Casting|CastToBP_Marine OtherActor))
  (Variables|/Game/Blueprints/Pawns/BP_Marine.BP_Marine_C|SetbOutsideMissionArea _asbp_marine false)
  (Utilities|Time|ClearTimerbyFunctionName 0 "KillPlayer"))

(event Collision|EventActorEndOverlap
  (params (OtherActor :type Actor%20Object%20Reference))
  (bind _asbp_marine (Utilities|Casting|CastToBP_Marine OtherActor))
  (Variables|/Game/Blueprints/Pawns/BP_Marine.BP_Marine_C|SetbOutsideMissionArea _asbp_marine true)
  (Utilities|Time|SetTimerbyFunctionName 0 "KillPlayer" (Variables|Default|GetSecondsBeforePlayerDeath)))

(fn ConstructionScript)

(fn KillPlayer
  (Game|Damage|ApplyDamage (Game|GetPlayerCharacter 0) 99999.0 0 0))